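; Bp_bulet is a short-lived bullet projectile actor that destroys itself half a second after spawning.
; Instead of overlap events, it runs a tiny sphere trace at its position every Tick, looking only for Vehicle objects.
; On a hit it hides both spheres, deactivates projectile movement, activates a shield-slam AOE effect component, then destroys itself after a brief delay.
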(event `self.ReceiveBeginPlay`
  (`KismetSystemLibrary.Delay` 0.5)
  (`self.K2_DestroyActor`))

(event `self.ReceiveTick`
  (params (DeltaSeconds :type "Float (single-precision)"))
  (bind _returnvalue (`self.K2_GetActorLocation`))
  (bind (_outhit _returnvalue_2) (`KismetSystemLibrary.SphereTraceSingleForObjects` _returnvalue (+ _returnvalue (1.0 0.0 0.0)) 1.0 (`|MakeArray` "ObjectTypeQuery5" :!type "EObjectTypeQuery Enum")))
  (if _returnvalue_2
    (`SceneComponent.SetVisibility` (`self.Sphere`) false false)
    (`ActorComponent.SetActive` (`self.ProjectileMovement`) false false)
    (`SceneComponent.SetVisibility` (`self.Sphere1`) false false)
    (`ActorComponent.SetActive` (`self.P_AU_ShieldSlam_AOE`) true false)
    (`KismetSystemLibrary.Delay` 0.4)
    (`self.K2_DestroyActor`)))

(fn `UserConstructionScript`)