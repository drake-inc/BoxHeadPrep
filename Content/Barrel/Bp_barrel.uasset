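; Explosive barrel actor that blows up when an AI_Zombie hits its mesh component.
; The hit spawns a large explosion particle plus Collision and Force actors at the barrel's location, then destroys the barrel.
; A separate overlap-style EventBang ignores the instigator, applies fixed damage to zombies and destroys the barrel on any other overlap.
; An unconnected copy of that damage logic targets Ai-enemy instead.
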(event `self.Barrel.OnComponentHit`
  (params (HitComponent :type "PrimitiveComponent Object Reference") (OtherActor :type "Actor Object Reference") (OtherComp :type "PrimitiveComponent Object Reference") (NormalImpulse :type "Vector Structure") (Hit :type "HitResult Structure (by ref)"))
  (bind _returnvalue (`SceneComponent.K2_GetComponentLocation` (`self.Barrel`)))
  (cast `/Game/Ai/AI_Zombie` OtherActor)
  (`GameplayStatics.SpawnEmitterAtLocation` "/Game/JunkWeCantDelete/P_Explosion.P_Explosion" _returnvalue (struct) (20.0 20.0 20.0))
  (`|SpawnActorFromClass` "/Game/ThirdPersonBP/Blueprints/ExplosionAttack/Collision.Collision_C" (`KismetMathLibrary.MakeTransform` _returnvalue) "Undefined" "OverrideRootScale" null null)
  (`|SpawnActorFromClass` "/Game/ThirdPersonBP/Blueprints/ExplosionAttack/Force.Force_C" (`KismetMathLibrary.MakeTransform` _returnvalue) "Undefined" "OverrideRootScale" null null)
  (`self.K2_DestroyActor`))

(event `EventBang`
  (params (OverlappedComponent :type "PrimitiveComponent Object Reference") (OtherActor :type "Actor Object Reference") (OtherComp :type "PrimitiveComponent Object Reference") (OtherBodyIndex :type Integer) (bFromSweep :type Boolean) (SweepResult :type "HitResult Structure (by ref)"))
  (if (!= OtherActor (`self.GetInstigator`))
    (bind _asai_zombie (cast `/Game/Ai/AI_Zombie` OtherActor)
      (:`then`
        (`GameplayStatics.ApplyDamage` _asai_zombie 34.0 null null "/Script/Engine.DamageType")
        (`self.K2_DestroyActor`))
      (:`CastFailed`
        (`self.K2_DestroyActor`)))))

(fn `UserConstructionScript`)