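; BP_powderexplosion is an explosive actor that detonates when a ThirdPersonCharacter overlaps its P_Explosion component.
; The overlap spawns an explosion emitter plus Collision and Force actors at the PExplosion location, then destroys the actor.
; A separate EventBang handler ignores the instigator, damages AI_Zombie hits and destroys itself on any other contact, with no binding shown.
; A disconnected copy targeting Ai-enemy never runs.
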(event `self.P_Explosion.OnComponentBeginOverlap`
  (params (OverlappedComponent :type "PrimitiveComponent Object Reference") (OtherActor :type "Actor Object Reference") (OtherComp :type "PrimitiveComponent Object Reference") (OtherBodyIndex :type Integer) (bFromSweep :type Boolean) (SweepResult :type "HitResult Structure (by ref)"))
  (bind _returnvalue (`SceneComponent.K2_GetComponentLocation` (`self.P_Explosion`)))
  (cast `/Game/Main_Charactter/ThirdPersonCharacter` OtherActor)
  (`GameplayStatics.SpawnEmitterAtLocation` "/Game/JunkWeCantDelete/P_Explosion.P_Explosion" _returnvalue)
  (`|SpawnActorFromClass` "/Game/ExplosionAttack/Collision.Collision_C" (`KismetMathLibrary.MakeTransform` _returnvalue) "Undefined" "OverrideRootScale" null null)
  (`|SpawnActorFromClass` "/Game/ExplosionAttack/Force.Force_C" (`KismetMathLibrary.MakeTransform` _returnvalue) "Undefined" "OverrideRootScale" null null)
  (`self.K2_DestroyActor`))

(event `EventBang`
  (params (OverlappedComponent :type "PrimitiveComponent Object Reference") (OtherActor :type "Actor Object Reference") (OtherComp :type "PrimitiveComponent Object Reference") (OtherBodyIndex :type Integer) (bFromSweep :type Boolean) (SweepResult :type "HitResult Structure (by ref)"))
  (if (!= OtherActor (`self.GetInstigator`))
    (bind _asai_zombie (cast `/Game/Ai/AI_Zombie` OtherActor)
      (:`then`
        (`GameplayStatics.ApplyDamage` _asai_zombie 34.0 null null "/Script/Engine.DamageType")
        (`self.K2_DestroyActor`))
      (:`CastFailed`
        (`self.K2_DestroyActor`)))))

(fn `UserConstructionScript`)