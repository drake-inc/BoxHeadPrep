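; Example melee sword actor that detects hits on enemies during attacks and shows a weapon trail.
; DetectStart begins the particle trail and runs a timeline that sphere-traces between the Start and End mesh sockets on each update; DetectStop ends both.
; Enemy-class hits receive a hit message with impact data and the parent actor's combat component state, then join an ignore list to prevent repeat hits.
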(event `DetectStart`
  (bind _returnvalue (`self.GetComponentByClass` (`self.GetParentActor`) "/Game/CombatSystem/CombatComponent.CombatComponent_C"))
  ;[1 1 1] Hit Detection
  (`ParticleSystemComponent.BeginTrails` (`self.ParticleSystem`) "Start" "End" "ETrailWidthMode_FromCentre" 1.0)
  (`KismetArrayLibrary.Array_Clear` (`self.Attacked`))
  (`Timeline|HitDetection` :!via `PlayFromStart` :!label _label
    (:`Update`
      (bind _outhit (`KismetSystemLibrary.SphereTraceSingle` (`SceneComponent.GetSocketLocation` (`self.StaticMesh`) "Start") (`SceneComponent.GetSocketLocation` (`self.StaticMesh`) "End") 15.0 "TraceTypeQuery1" false (`self.Attacked`)))
      (if (`KismetMathLibrary.ClassIsChildOf` (`GameplayStatics.GetObjectClass` (`.HitActor` (`GameplayStatics.BreakHitResult` _outhit))) (`self.EnemyClass`))
        (message `/Game/CombatSystem/CombatInterface.SuccesssfulHit` (`.HitActor` (`GameplayStatics.BreakHitResult` _outhit)) (`/Game/CombatSystem/CombatComponent.CurrentCombo` _returnvalue) (`/Game/CombatSystem/CombatComponent.CurrentAnim` _returnvalue) (`/Game/CombatSystem/CombatComponent.CurrentWeapon` _returnvalue) 1 (`.ImpactPoint` (`GameplayStatics.BreakHitResult` _outhit)) (`.ImpactNormal` (`GameplayStatics.BreakHitResult` _outhit)) (`.HitBoneName` (`GameplayStatics.BreakHitResult` _outhit)) (`self.GetParentActor`))
        (`KismetArrayLibrary.Array_Add` (`self.Attacked`) (`.HitActor` (`GameplayStatics.BreakHitResult` _outhit)))))))

(event `DetectStop`
  ;[1 1 1] Hit Detection
  (`ParticleSystemComponent.EndTrails` (`self.ParticleSystem`))
  (`KismetArrayLibrary.Array_Clear` (`self.Attacked`))
  (goto _label :!via `Stop`))

(fn `UserConstructionScript`)